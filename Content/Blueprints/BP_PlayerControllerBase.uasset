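; Base player controller for mouse-driven movement on a grid.
; A left click traces under the cursor for a grid cell and asks the game controller to move the player pawn there from the player's current cell.
; A timer advanced on Tick enforces a cooldown between successful moves.
; Tick also traces under the cursor, clearing the grid's hover sprites and highlighting the hovered cell.
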(event EventTick
  (params (DeltaSeconds :type Float%20%28single-precision%29))
  (bind (_hitresult _returnvalue) (Game|Player|GetHitResultUnderCursorbyChannel "TraceTypeQuery1" true))
  (Variables|Default|SettimeSinceLastMove (+ (Variables|Default|GettimeSinceLastMove) DeltaSeconds))
  ;[1 1 1] Paints the cell a differente color on mouse hover
  (if _returnvalue
    (bind _asbp_grid_cell_base (Utilities|Casting|CastToBP_GridCellBase (.HitActor (Collision|BreakHitResult _hitresult))))
    (bind _returnvalue_2 (Actor|GetActorOfClass "/Game/Blueprints/BP_GridBase.BP_GridBase_C"))
    (Default|ClearAllHoverSprites _returnvalue_2)
    (Default|SetHoverSprite _asbp_grid_cell_base)))

(event Input|MouseEvents|LeftMouseButton
  (params (Key :type Key%20Structure :default "None"))
  (bind (_hitresult _returnvalue) (Game|Player|GetHitResultUnderCursorbyChannel "TraceTypeQuery1" true))
  (:Pressed
    (if (> (Variables|Default|GettimeSinceLastMove) (Variables|Default|GetmoveCooldown))
      (if _returnvalue
        (bind _asbp_grid_cell_base (Utilities|Casting|CastToBP_GridCellBase (.HitActor (Collision|BreakHitResult _hitresult))))
        (bind _output_get (Variables|Default|SetClickedSquare _asbp_grid_cell_base))
        (bind _outactors (Actor|GetAllActorsOfClass "/Game/Blueprints/BP_GameControllerBase.BP_GameControllerBase_C"))
        (bind _asbp_game_controller_base (Utilities|Casting|CastToBP_GameControllerBase (Utilities|Array|Get(acopy) _outactors)))
        (bind _returnvalue_2 (Actor|GetActorOfClass "/Game/Blueprints/BP_PlayerBase.BP_PlayerBase_C"))
        (bind _moved (Default|MoveCharacter _asbp_game_controller_base _output_get false (Game|Player|GetPlayerPawn 0) true (Variables|/Game/Blueprints/BP_PlayerBase.BP_PlayerBase_C|GetcurrentCell _returnvalue_2)))
        (if _moved
          (Variables|Default|SettimeSinceLastMove 0.0))))))

(fn ConstructionScript)