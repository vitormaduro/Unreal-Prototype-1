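; BP_PlayerBase is a base player Blueprint that switches a Paper2D flipbook between idle and jump animations.
; UpdateAnimation picks the flipbook from the IsJumping flag, which nothing in this file sets to true.
; Tick times an active jump, then clears the flag after one second and refreshes the animation.
; BeginPlay shows the mouse cursor for the first player controller.
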(event Custom|UpdateAnimation
  (if (Variables|Default|GetisJumping)
    (Sprite|SetFlipbook (Variables|Default|GetPaperFlipbook) (Variables|Default|GetjumpFlipbook))
    (else
      (Sprite|SetFlipbook (Variables|Default|GetPaperFlipbook) (Variables|Default|GetidleFlipbook)))))

(event EventBeginPlay
  (Variables|/Script/Engine.PlayerController|SetbShowMouseCursor (Game|GetPlayerController 0) true))

(event Collision|EventActorBeginOverlap
  (params (OtherActor :type Actor%20Object%20Reference)))

(event EventTick
  (params (DeltaSeconds :type Float%20%28single-precision%29))
  (if (Variables|Default|GetisJumping)
    (Variables|Default|SetjumpTime (+ DeltaSeconds (Variables|Default|GetjumpTime)))
    (if (>= (Variables|Default|GetjumpTime) 1.0)
      (Variables|Default|SetjumpTime 0.0)
      (Variables|Default|SetisJumping false)
      (CallFunction|UpdateAnimation))))

(fn ConstructionScript)