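; BP_GridBase is a grid base actor that creates and tracks the cells of a square grid.
; AddGridSquare spawns a BP_GridCellBase at a given transform, stores it in CellsArray, marks it free and coinless, and derives its two-part ID from array index and grid width.
; ClearAllHoverSprites loops over the stored cells and calls SetSprite to clear hover visuals.
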(event EventBeginPlay)

(event Collision|EventActorBeginOverlap
  (params (OtherActor :type Actor%20Object%20Reference)))

(event EventTick
  (params (DeltaSeconds :type Float%20%28single-precision%29)))

(fn ConstructionScript)

(fn AddGridSquare
  (params (square%20transform :type Transform) (gridWidth :type Integer))
  (bind _returnvalue (Game|SpawnActorfromClass "/Game/Blueprints/BP_GridCellBase.BP_GridCellBase_C" square%20transform "Undefined" 0 0))
  (bind _returnvalue_2 (Utilities|Array|Add (Variables|Default|GetcellsArray) _returnvalue))
  (Variables|/Script/PUGA_game.GridCellBase|SetisFree _returnvalue true)
  (Variables|/Script/PUGA_game.GridCellBase|SethasCoin _returnvalue false)
  (Class|GridCellBase|SetId _returnvalue (Utilities|Array|MakeArray (/ _returnvalue_2 gridWidth) (Math|Integer|%(Integer) _returnvalue_2 gridWidth))))

(fn ClearAllHoverSprites
  (for _array_element (Variables|Default|GetcellsArray)
    (bind _asbp_grid_cell_base (Utilities|Casting|CastToBP_GridCellBase _array_element))
    (Default|SetSprite _asbp_grid_cell_base)))