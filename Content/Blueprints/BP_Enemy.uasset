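; BP_Enemy is a flipbook-animated enemy that hops between grid cells on a randomized cooldown.
; When the cooldown expires, it gets valid cells from the game controller, has EnemyAIBase pick the next path cell using the coin cells, then requests a forced move.
; A successful move rerolls the cooldown.
; A separate repeating timer clears the jumping flag and refreshes animation, though both animation branches set the jump flipbook.
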(event Custom|Update%20Animation
  (if (Variables|Default|GetisJumping)
    (Sprite|SetFlipbook (Variables|Default|GetPaperFlipbook) (Variables|Default|GetjumpFlipbook))
    (else
      (Sprite|SetFlipbook (Variables|Default|GetPaperFlipbook) (Variables|Default|GetjumpFlipbook)))))

(event EventBeginPlay
  (bind _returnvalue (Actor|GetActorOfClass "/Game/Blueprints/BP_GameControllerBase.BP_GameControllerBase_C"))
  (Variables|Default|SetGameController _returnvalue))

(event EventTick
  (params (DeltaSeconds :type Float%20%28single-precision%29))
  (bind _gamecontroller (Variables|Default|GetGameController))
  (Variables|Default|SetjumpTime (+ (Variables|Default|GetjumpTime) DeltaSeconds))
  (if (>= (Variables|Default|GetjumpTime) 1.0)
    (Variables|Default|SetjumpTime 0.0)
    (Variables|Default|SetisJumping false)
    (CallFunction|UpdateAnimation))
  (Variables|Default|SetTimeSinceLastJump (+ DeltaSeconds (Variables|Default|GetTimeSinceLastJump)))
  (if (>= (Variables|Default|GetTimeSinceLastJump) (Variables|Default|GetCurrentJumpCooldown))
    (Actor|GetActorOfClass "/Game/Blueprints/BP_GridBase.BP_GridBase_C")
    (bind _returnvalue (Class|GameControllerBase|GetValidCells _gamecontroller (Variables|Default|GetPosition)))
    (bind _returnvalue_2 (Class|EnemyAIBase|GetNextCellinPath (Variables|Default|GetEnemyAIBase) _returnvalue self (Variables|/Game/Blueprints/BP_GameControllerBase.BP_GameControllerBase_C|GetCellsWithCoins _gamecontroller)))
    (bind _asbp_grid_cell_base (Utilities|Casting|CastToBP_GridCellBase _returnvalue_2))
    (bind _square (Default|GetSquarebyId (Variables|Default|GetGameController) (Variables|Default|GetPosition)))
    (bind _moved (Default|MoveCharacter (Variables|Default|GetGameController) _asbp_grid_cell_base true self false _square))
    (if _moved
      (Variables|Default|SetTimeSinceLastJump 0.0)
      (Variables|Default|SetCurrentJumpCooldown (Math|Random|RandomFloatinRange (Variables|Default|GetMinTimeBetweenJumps) (Variables|Default|GetMaxTimeBetweenJumps))))))

(fn ConstructionScript)