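; BP_GridCellBase is a base actor for a single grid cell, shown with a Paper2D sprite that reflects whether the cell is valid.
; ToggleSprite flips the Valid flag and swaps between the invalid and valid entries of the Sprites array.
; SetHoverSprite shows a separate hover sprite, and SetSprite restores the one matching the current Valid state.
; Its event graph and construction script are empty, so these functions only run when called.
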(event EventBeginPlay)

(event Collision|EventActorBeginOverlap
  (params (OtherActor :type Actor%20Object%20Reference)))

(event EventTick
  (params (DeltaSeconds :type Float%20%28single-precision%29)))

(fn ConstructionScript)

(fn ToggleSprite
  (if (Variables|Default|GetValid)
    (Rendering|Components|Sprite|SetSprite (Variables|Default|GetPaperSprite) (Utilities|Array|Get(acopy) (Variables|Default|GetSprites)))
    (Variables|Default|SetValid false)
    (else
      (Rendering|Components|Sprite|SetSprite (Variables|Default|GetPaperSprite) (Utilities|Array|Get(acopy) (Variables|Default|GetSprites) 1))
      (Variables|Default|SetValid true))))

(fn SetHoverSprite
  (Rendering|Components|Sprite|SetSprite (Variables|Default|GetPaperSprite) (Utilities|Array|Get(acopy) (Variables|Default|GetSprites) 2)))

(fn SetSprite
  (if (Variables|Default|GetValid)
    (Rendering|Components|Sprite|SetSprite (Variables|Default|GetPaperSprite) (Utilities|Array|Get(acopy) (Variables|Default|GetSprites) 1))
    (else
      (Rendering|Components|Sprite|SetSprite (Variables|Default|GetPaperSprite) (Utilities|Array|Get(acopy) (Variables|Default|GetSprites))))))